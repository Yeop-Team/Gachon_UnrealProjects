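; BP_Ey_Bu is a projectile, apparently an enemy bullet, that damages the player on contact.
; Each tick it moves along Direction at Speed by setting its location without sweep.
; On collision overlap it reads SelectedColor from BP_GameInstance to choose whether to cast to the red or blue player.
; A matching player takes fixed damage, then the projectile plays a blaster sound and destroys itself.
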(event `self.ReceiveTick`
  (params (DeltaSeconds :type "Float (single-precision)"))
  ; 이동한다.
  (`self.K2_SetActorLocation` (+ (* DeltaSeconds (* (`self.Direction`) (`self.Speed`))) (`self.K2_GetActorLocation`))))

(event `self.Collision.OnComponentBeginOverlap`
  (params (OverlappedComponent :type "PrimitiveComponent Object Reference") (OtherActor :type "Actor Object Reference") (OtherComp :type "PrimitiveComponent Object Reference") (OtherBodyIndex :type Integer) (bFromSweep :type Boolean) (SweepResult :type "HitResult Structure (by ref)"))
  (bind _asbp_game_instance (cast `/Game/Blueprints/BP_GameInstance` (`GameplayStatics.GetGameInstance`)))
  (switch `string` (`/Game/Blueprints/BP_GameInstance.SelectedColor` _asbp_game_instance)
    (:`Red`
      (bind _asbp_player_red (cast `/Game/Blueprints/BP_Player_Red` OtherActor))
      (`/Game/Blueprints/BP_Player_Red.데미지` _asbp_player_red 20)
      (`GameplayStatics.PlaySound2D` "/Game/star-wars-blaster.star-wars-blaster" 1.0 1.0 0.0 null null)
      (`self.K2_DestroyActor`))
    (:`Blue`
      (bind _asbp_player_blue (cast `/Game/Blueprints/BP_Player_Blue` OtherActor))
      (`/Game/Blueprints/BP_Player_Blue.데미지` _asbp_player_blue 20)
      (`GameplayStatics.PlaySound2D` "/Game/star-wars-blaster.star-wars-blaster" 1.0 1.0 0.0 null null)
      (`self.K2_DestroyActor`))))

(fn `UserConstructionScript`)